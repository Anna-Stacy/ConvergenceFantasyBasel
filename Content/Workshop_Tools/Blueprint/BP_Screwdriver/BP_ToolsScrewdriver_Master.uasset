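; BP_ToolsScrewdriver_Master is a configurable screwdriver prop for the workshop tools set, with selectable body and bit meshes.
; Its construction script picks meshes from two arrays using the ScrewdriverVariants and BitVariants selectors and applies them to the matching static mesh components.
; The event graph holds only disabled default events, so it has no runtime behavior.
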(event EventBeginPlay)

(event Collision|EventActorBeginOverlap
  (params (OtherActor :type Actor%20Object%20Reference)))

(event EventTick
  (params (DeltaSeconds :type Float%20%28single-precision%29)))

(fn ConstructionScript
  (bind _var (Variables|Default|GetVar))
  (bind _newvar_0 (Variables|Default|GetNewVar_0))
  (Utilities|Array|SetArrayElem _var 0 "/Game/Workshop_Tools/Meshes/Screwdriver/SM_ToolsScrewdriverNozzleBitSocket.SM_ToolsScrewdriverNozzleBitSocket")
  (Components|StaticMesh|SetStaticMesh (Variables|Default|GetScrewdriver_Variants) (Utilities|Array|Get(acopy) _var (Variables|Default|GetScrewdriverVariants)))
  (Utilities|Array|SetArrayElem _newvar_0 0 0)
  (Components|StaticMesh|SetStaticMesh (Variables|Default|GetBit_Variants) (Utilities|Array|Get(acopy) _newvar_0 (Variables|Default|GetBitVariants))))