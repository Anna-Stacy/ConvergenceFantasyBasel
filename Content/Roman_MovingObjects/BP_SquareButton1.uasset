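; BP_SquareButton1 is a configurable square button with a cube touch sensor, a four-sided border and a text label.
; Its construction script calls the parent, scales the sensor from ButtonSizeInCm and stores that size in SensorTouchVolume.
; The same size scales and positions the border bars, offset by BorderBackdrop, while exposed variables style the border and label.
; The event graph is inactive, so this Blueprint only builds the button's layout.
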(event EventBeginPlay
  (|CallParentFunction) ; This node is disabled and will not be called.\nDrag off pins to build functionality.
)

(event Collision|EventActorBeginOverlap
  (params (OtherActor :type Actor%20Object%20Reference))
  (|CallParentFunction OtherActor) ; This node is disabled and will not be called.\nDrag off pins to build functionality.
)

(event EventTick
  (params (DeltaSeconds :type Float%20%28single-precision%29))
  (|CallParentFunction DeltaSeconds) ; This node is disabled and will not be called.\nDrag off pins to build functionality.
)

(fn ConstructionScript
  (bind _buttonsize_in_cm (Variables|Default|GetButtonSize%20in%20cm))
  (bind _touchsensor (Variables|Default|GetTouchSensor))
  (bind _buttonsize_in_cm_2 (Variables|Default|GetButtonSize%20in%20cm))
  (bind _buttontextmarking (Variables|Default|GetButtonTextMarking))
  (bind _bordertop (Variables|Default|GetBorderTop))
  (bind _borderbottom (Variables|Default|GetBorderBottom))
  (bind _borderleft (Variables|Default|GetBorderLeft))
  (bind _borderright (Variables|Default|GetBorderRight))
  (|CallParentFunction)
  (Utilities|FlowControl|Sequence
    (:then_0
      ;[1 1 1] Define Sensor as a cube with a given size
      (Components|StaticMesh|SetStaticMesh _touchsensor "/Engine/EngineMeshes/Cube.Cube")
      (Transformation|SetWorldScale3D _touchsensor (/ _buttonsize_in_cm "250.000000,250.000000,250.000000"))
      (Variables|Default|SetSensorTouchVolume _buttonsize_in_cm))
    (:then_1
      ;[1 1 1] Create Button Border
      (Transformation|SetWorldScale3D _bordertop (* _buttonsize_in_cm_2 "0.010000,0.011500,0.000500"))
      (Transformation|SetRelativeLocation _bordertop (+ (* _buttonsize_in_cm_2 "0.000000,0.000000,0.550000") (Math|Vector|MakeVector (Variables|Default|GetBorderBackdrop) 0.0 0.0)) false false)
      (Transformation|SetWorldScale3D _borderbottom (* _buttonsize_in_cm_2 "0.010000,0.011500,0.000500"))
      (Transformation|SetRelativeLocation _borderbottom (+ (* _buttonsize_in_cm_2 "0.000000,0.000000,-0.550000") (Math|Vector|MakeVector (Variables|Default|GetBorderBackdrop) 0.0 0.0)) false false)
      (Transformation|SetWorldScale3D _borderleft (* _buttonsize_in_cm_2 "0.010000,0.000500,0.011000"))
      (Transformation|SetRelativeLocation _borderleft (+ (* _buttonsize_in_cm_2 "0.000000,0.550000,0.000000") (Math|Vector|MakeVector (Variables|Default|GetBorderBackdrop) 0.0 0.0)) false false)
      (Transformation|SetWorldScale3D _borderright (* _buttonsize_in_cm_2 "0.010000,0.000500,0.011000"))
      (Transformation|SetRelativeLocation _borderright (+ (* _buttonsize_in_cm_2 "0.000000,-0.550000,0.000000") (Math|Vector|MakeVector (Variables|Default|GetBorderBackdrop) 0.0 0.0)) false false)
      (Rendering|Material|SetMaterial (Variables|Default|GetBorderRight) 0 (Variables|Default|GetBorderMaterial)))
    (:then_2
      (Rendering|Components|TextRender|SetText _buttontextmarking (Variables|Default|GetButtonText))
      (Rendering|Components|TextRender|SetWorldSize _buttontextmarking (Variables|Default|GetTextSize))
      (Rendering|Components|TextRender|SetTextRenderColor _buttontextmarking (Variables|Default|GetTextColor)))))