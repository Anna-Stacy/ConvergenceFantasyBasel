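; Networked VR user platform actor that serves as the shared play-area floor and movement base for all players.
; It reads boundary settings from VR_GameState and sizes the plane plus inner and outer chaperone walls, shown by headset proximity unless inner walls are always visible.
; VR offset updates teleport the platform and re-align every pawn.
; It also toggles players' local head visibility and cycles supervisor camera target transforms.
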(event Custom|SetupChaperones
  (bind _user_area_base_dimension (Variables|Chaperones|GetUser%20Area%20Base%20Dimension))
  (Transformation|SetWorldScale3D (Variables|Default|GetPlane) (Math|Vector|MakeVector (.x _user_area_base_dimension) (.y _user_area_base_dimension) 1.0))
  (|SetupInnerChaperones)
  (|SetupOuterChaperones))

(event Custom|SR_Make%20all%20Heads%20visible
  ;[1 0.4 0.4] Make local player head visible, when coming back to the lobby (Mirror).
  (for _array_element (Variables|/Game/VR_Base/VR_GameState.VR_GameState_C|GetList%20of%20all%20Players (.AsVR%20Game%20State (Utilities|Casting|CastToVR_GameState (Game|GetGameState))))
    (bind _asvr_pawn (Utilities|Casting|CastToVR_Pawn _array_element))
    (Default|SRMakeHeadVisible _asvr_pawn)))

(event Custom|SR_Hide%20all%20local%20Heads
  ;[1 0.4 0.4] Hide local player head, when leaving the lobby (No more Mirrors).
  (for _array_element (Variables|/Game/VR_Base/VR_GameState.VR_GameState_C|GetList%20of%20all%20Players (.AsVR%20Game%20State (Utilities|Casting|CastToVR_GameState (Game|GetGameState))))
    (bind _asvr_pawn (Utilities|Casting|CastToVR_Pawn _array_element))
    (Default|SRHideLocalHead _asvr_pawn)))

(event Custom|OC_CheckChaperones
  (params (HDM :type Vector) (VR_Pawn :type VR%20Pawn%20Object%20Reference))
  (bind (_x _y) (Math|Vector|BreakVector HDM))
  (bind _user_area_base_dimension (Variables|Chaperones|GetUser%20Area%20Base%20Dimension))
  (bind (_x_2 _y_2) (Math|Vector|BreakVector _user_area_base_dimension))
  ;[0.4 1 0.4] Only apply it locally, and if chaperones are not already always visible
  (if (and (not (Variables|Chaperones|GetChaperonesAlwaysVisible)) (Variables|Chaperones|GetChaperonesActive))
    ;[0.4 1 0.4] Set dynamic chaperone visibility in X-Plus direction
    (Rendering|SetVisibility (Variables|Default|GetInner_Chaperone_X_Plus) (> _x (- (* _x_2 5e+01) (Variables|Chaperones|GetChaperonesWarningDistance))) true)
    (Rendering|SetVisibility (Variables|Default|GetOuter_Chaperone_X_Plus) (> _x (- (* _x_2 5e+01) (Variables|Chaperones|GetGoBackWarningDistance))) true)
    ;[0.4 1 0.4] Set dynamic chaperone visibility in X-Minus direction
    (Rendering|SetVisibility (Variables|Default|GetInner_Chaperone_X_Minus) (< _x (+ (* _x_2 -5e+01) (Variables|Chaperones|GetChaperonesWarningDistance))) true)
    (Rendering|SetVisibility (Variables|Default|GetOuter_Chaperone_X_Minus) (< _x (+ (* _x_2 -5e+01) (Variables|Chaperones|GetGoBackWarningDistance))) true)
    ;[0.4 1 0.4] Set dynamic chaperone visibility in Y-Plus direction
    (Rendering|SetVisibility (Variables|Default|GetInner_Chaperone_Y_Plus) (> _y (- (* _y_2 5e+01) (Variables|Chaperones|GetChaperonesWarningDistance))) true)
    (Rendering|SetVisibility (Variables|Default|GetOuter_Chaperone_Y_Plus) (> _y (- (* _y_2 5e+01) (Variables|Chaperones|GetGoBackWarningDistance))) true)
    ;[0.4 1 0.4] Set dynamic chaperone visibility in Y-Minus direction
    (Rendering|SetVisibility (Variables|Default|GetInner_Chaperone_Y_Minus) (< _y (+ (* _y_2 -5e+01) (Variables|Chaperones|GetChaperonesWarningDistance))) true)
    (Rendering|SetVisibility (Variables|Default|GetOuter_Chaperone_Y_Minus) (< _y (+ (* _y_2 -5e+01) (Variables|Chaperones|GetGoBackWarningDistance))) true)))

(event EventBeginPlay
  ;[1 1 0.4 1 36] BeginPlay
  (|CallParentFunction)
  (Actor|Tick|SetActorTickEnabled true)
  (Development|PrintString "Event BeginPlay" false)
  (CallFunction|SetDebugVariable)
  (Networking|SwitchHasAuthority
    (:Authority
      ;;[1 1 1] Setup variables
      (bind _asvr_game_state (Utilities|Casting|CastToVR_GameState (Game|GetGameState)))
      (Variables|Chaperones|SetChaperonesActive (Variables|/Game/VR_Base/VR_GameState.VR_GameState_C|GetChaperonesActive _asvr_game_state))
      (Variables|Chaperones|SetChaperonesAlwaysVisible (Variables|/Game/VR_Base/VR_GameState.VR_GameState_C|GetChaperonesAlwaysVisible _asvr_game_state))
      (Variables|Chaperones|SetChaperonesWarningDistance (Variables|/Game/VR_Base/VR_GameState.VR_GameState_C|GetChaperonesWarningDistance _asvr_game_state))
      (Variables|Chaperones|SetGoBackWarningDistance (Variables|/Game/VR_Base/VR_GameState.VR_GameState_C|GetGoBackWarningDistance _asvr_game_state))
      (Variables|Chaperones|SetInnerToOuterChaperoneDistance (Variables|/Game/VR_Base/VR_GameState.VR_GameState_C|GetInnerToOuterChaperonesDistance _asvr_game_state))
      (Variables|Chaperones|SetUser%20Area%20Base%20Dimension (Variables|/Game/VR_Base/VR_GameState.VR_GameState_C|GetUserAreaBaseDimension _asvr_game_state)))
    (:Remote
      (Class|GameplayStatics|SetBaseSoundMix "/Game/VR_Base/Streaming/SMix_General.SMix_General"))))

(fn ConstructionScript
  (|CallParentFunction)
  (bind _asvr_game_state (Utilities|Casting|CastToVR_GameState (Game|GetGameState)))
  (Variables|Chaperones|SetChaperonesActive (Variables|/Game/VR_Base/VR_GameState.VR_GameState_C|GetChaperonesActive _asvr_game_state))
  (Variables|Chaperones|SetChaperonesAlwaysVisible (Variables|/Game/VR_Base/VR_GameState.VR_GameState_C|GetChaperonesAlwaysVisible _asvr_game_state))
  (Variables|Chaperones|SetChaperonesWarningDistance (Variables|/Game/VR_Base/VR_GameState.VR_GameState_C|GetChaperonesWarningDistance _asvr_game_state))
  (Variables|Chaperones|SetGoBackWarningDistance (Variables|/Game/VR_Base/VR_GameState.VR_GameState_C|GetGoBackWarningDistance _asvr_game_state))
  (Variables|Chaperones|SetInnerToOuterChaperoneDistance (Variables|/Game/VR_Base/VR_GameState.VR_GameState_C|GetInnerToOuterChaperonesDistance _asvr_game_state))
  (Variables|Chaperones|SetUser%20Area%20Base%20Dimension (Variables|/Game/VR_Base/VR_GameState.VR_GameState_C|GetUserAreaBaseDimension _asvr_game_state))
  (bind _output_get (Variables|Default|SetDebugStartup (Variables|/Game/VR_Base/VR_GameState.VR_GameState_C|GetDebug%20Startup _asvr_game_state)))
  (Utilities|PrintDebugMessage "End of Construction Script" "NewEnumerator0" _output_get))

(fn UpdateVROffset
  (params (VROffset :type Vector))
  (Utilities|FlowControl|Sequence
    (:then_0
      ;[1 1 1] Change BP_StreamingSystem Plane location
      (Transformation|SetActorLocation VROffset true true))
    (:then_1
      ;[1 1 1] Adjust all Player capsules to the new Plane as their Character Movement Base
      (|ReportTravel_2 VROffset)
      (for _array_element (Variables|/Game/VR_Base/VR_GameState.VR_GameState_C|GetList%20of%20all%20Players (.AsVR%20Game%20State (Utilities|Casting|CastToVR_GameState (Game|GetGameState))))
        (bind _asvr_pawn (Utilities|Casting|CastToVR_Pawn _array_element))
        (Default|SRSetWorldLocation _asvr_pawn)))))

(fn SetChaperonesAlwaysVisible
  (params (ChaperonesAlwaysVisible :type Boolean))
  (Variables|Chaperones|SetChaperonesAlwaysVisible ChaperonesAlwaysVisible))

(fn OnRepChaperonesAlwaysVisible
  (Rendering|SetVisibility (Variables|Default|GetInnerChaperones) (Variables|Chaperones|GetChaperonesAlwaysVisible) true))

(fn SetDebugVariable
  (bind _asvr_game_state (Utilities|Casting|CastToVR_GameState (Game|GetGameState)))
  (Variables|Default|SetDebug%20Travel (Math|Boolean|ORBoolean (Variables|/Game/VR_Base/VR_GameState.VR_GameState_C|GetDebugTeleport _asvr_game_state) (Variables|/Game/VR_Base/VR_GameState.VR_GameState_C|GetDebugTravel _asvr_game_state) (Variables|/Game/VR_Base/VR_GameState.VR_GameState_C|GetDebugContinuousTravel _asvr_game_state))))

(fn OnRepVROffset
  (Utilities|FlowControl|Sequence
    (:then_0
      ;[1 1 1] Change BP_StreamingSystem Plane location
      (Transformation|SetActorLocation (Variables|Default|GetVROffset) true true))
    (:then_1
      ;[1 1 1] Adjust all Player capsules to the new Plane as their Character Movement Base
      (|ReportTravel_2_2 (Variables|Default|GetVROffset))
      (for _array_element (Variables|/Game/VR_Base/VR_GameState.VR_GameState_C|GetList%20of%20all%20Players (.AsVR%20Game%20State (Utilities|Casting|CastToVR_GameState (Game|GetGameState))))
        (bind _asvr_pawn (Utilities|Casting|CastToVR_Pawn _array_element))
        (Default|SRSetWorldLocation _asvr_pawn)))))

(fn SwitchCameraView
  (params (Increment :type Boolean))
  (bind _supervisorcameratransforms (Variables|Supervisor|GetSupervisorCameraTransforms))
  (bind _returnvalue (Utilities|Array|Length _supervisorcameratransforms))
  ;[1 1 1] Check if cams are defined
  (if (> _returnvalue 0)
    ;[1 1 1] Calc max camera index
    (LocalVariables|SetMaxCameraIndex (- _returnvalue 1))
    (Utilities|FlowControl|Sequence
      (:then_0
        (if Increment
          ;[1 1 1] Increment and wrap around to zero if exceeding max index
          (Variables|Supervisor|SetCurrentCameraTransformIndex (Math|Integer|SelectInt (+ (Variables|Supervisor|GetCurrentCameraTransformIndex) 1) 0 (<= (+ (Variables|Supervisor|GetCurrentCameraTransformIndex) 1) (LocalVariables|GetMaxCameraIndex))))
          (else
            ;[1 1 1] Decrement and wrap around to max index if less then zero
            (Variables|Supervisor|SetCurrentCameraTransformIndex (Math|Integer|SelectInt (- (Variables|Supervisor|GetCurrentCameraTransformIndex) 1) (LocalVariables|GetMaxCameraIndex) (>= (- (Variables|Supervisor|GetCurrentCameraTransformIndex) 1) 0))))))
      (:then_1
        ;[1 1 1] Change camera target transform
        (Variables|Supervisor|SetShouldLerpCamera true)
        (bind _output_get (Variables|Supervisor|SetTargetTransform (Utilities|Array|Get(acopy) (Variables|Supervisor|GetSupervisorCameraTransforms) (Variables|Supervisor|GetCurrentCameraTransformIndex))))
        (|Reportcamerachange _output_get (Variables|Supervisor|GetCurrentCameraTransformIndex))))
    (else
      (Utilities|PrintDebugMessage "No Supervisor camera definitions found" "NewEnumerator2" true))))

(fn GetCameraTransformsforCurrentLevel
  (return (Variables|Supervisor|GetSupervisorCameraTransforms)))

(fn OnRepPlayfieldBaseDimension
  (CallFunction|SetupChaperones))

(fn OnRepUserAreaBaseDimension
  (CallFunction|SetupChaperones))