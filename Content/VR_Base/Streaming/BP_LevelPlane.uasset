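; BP_LevelPlane is a labelled plane actor in the VR streaming setup that displays a level name.
; The construction script writes LevelName to its text render and sets the plane's visibility from PlaneVisibility.
; When the VR_GameState streaming debug flag is on, BeginPlay waits briefly for init, then prints BP_StreamingSystem's current level or reports that actor missing.
; It only reports streaming state and does no loading itself.
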(event EventBeginPlay
  ;[1 1 0.4] Initialization
  (bind _asvr_game_state (Utilities|Casting|CastToVR_GameState (Game|GetGameState)))
  (bind _output_get (Variables|Default|SetDebug (Variables|/Game/VR_Base/VR_GameState.VR_GameState_C|GetDebugStreaming _asvr_game_state)))
  (if _output_get
    (Utilities|FlowControl|Delay 0.2) ; Wait for init to finish
    (bind _returnvalue (Actor|GetActorOfClass "/Game/VR_Base/Streaming/BP_StreamingSystem.BP_StreamingSystem_C"))
    (Utilities|IsValid _returnvalue
      (:Is%20Valid
        (Development|PrintString (Utilities|String|Append "Current Streaming State is " (Utilities|String|ToString(Name) (Variables|/Game/VR_Base/Streaming/BP_UserPlatform.BP_UserPlatform_C|GetCurrent%20Level _returnvalue))) (Variables|Default|GetDebug) true "(R=0.000000,G=0.660000,B=1.000000,A=1.000000)" 1e+01))
      (:Is%20Not%20Valid
        (Development|PrintString "Missing BP_StreamingSystem actor" (Variables|Default|GetDebug))))))

(fn ConstructionScript
  (Rendering|Components|TextRender|SetText (Variables|Default|GetTextRender) (Utilities|Text|ToText(Name) (Variables|Default|GetLevelName)))
  (Rendering|SetVisibility (Variables|Default|GetPlane) (Variables|Default|GetPlaneVisibility) false)
  (bind _asvr_game_state (Utilities|Casting|CastToVR_GameState (Game|GetGameState)))
  (Development|PrintString "End of Construction Script" (Variables|/Game/VR_Base/VR_GameState.VR_GameState_C|GetDebug%20Startup _asvr_game_state) (Variables|/Game/VR_Base/VR_GameState.VR_GameState_C|GetDebug%20Startup _asvr_game_state)))