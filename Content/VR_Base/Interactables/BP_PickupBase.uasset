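; Base actor for replicated VR pickups that players grab and drop, with critical objects able to respawn at their original spot.
; The server attaches the mesh to the hand with per-hand offsets, while RepNotify toggles physics.
; It finds the streaming system, optionally attaches to it, and stores its initial transform relative to it.
; Respawn multicasts a timer-driven blink before teleporting back, which pickup cancels; subclass hooks are left empty.
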(event Custom|AttachToStreamingSystem
  (params (NewLevel :type Name))
  ;[1 1 1] Attaching object to streaming system
  (Utilities|FlowControl|Sequence
    (:then_0
      (if (Variables|Default|GetShouldAttachToStreamingSystem)
        (Transformation|AttachActorToActor (Variables|ObjectRespawn|GetStreamingSystemRef) "None" "KeepWorld" "KeepWorld" "KeepWorld" true)))
    (:then_1
      (Variables|ObjectRespawn|SetInitialTransform (Math|Transform|MakeRelativeTransform (Transformation|GetActorTransform) (Transformation|GetActorTransform (Variables|ObjectRespawn|GetStreamingSystemRef)))))))

(event Custom|MC_StartBlinkThenRespawnObject
  ;[0.4 0.7 1 0.5] Multicast Respawn
  (Variables|ObjectRespawn|SetBlinkCounter 0)
  (bind _returnvalue (Utilities|Time|SetTimerbyFunctionName 0 "BlinkObjectThenRespawn" 0.3 true))
  (Variables|ObjectRespawn|SetBlinkHandle _returnvalue))

(event Custom|ResetStateForRespawn
  ;[1 0.4 0.4] Called on Server - called by timer
)

(event Custom|Multicast_CancelRespawn
  ;[0.4 0.7 1 0.5] Multicast Cancel Respawn
  (Rendering|SetActorHiddenInGame false)
  (Utilities|Time|ClearandInvalidateTimerbyHandle (Variables|ObjectRespawn|GetBlinkHandle)))

(event Custom|Respawn
  ;[1 0.4 0.4] Setting up "respawning" of important objects, moving them back to original location
  (Networking|SwitchHasAuthority
    (:Authority
      (if (Variables|ObjectRespawn|GetIsCriticalObject)
        (if (> (Variables|ObjectRespawn|GetDelayBeforeRespawn) 0.0)
          (Utilities|FlowControl|Delay (Variables|ObjectRespawn|GetDelayBeforeRespawn)))
        (if (and (not (Variables|Pickup|GetIsPickedUp)) (not (Variables|ObjectRespawn|GetJustRespawned)))
          (Variables|Default|SetShouldSimulatePhysics false)
          (Variables|ObjectRespawn|SetJustRespawned true)
          (CallFunction|MCStartBlinkThenRespawnObject))
        (else
          (Variables|ObjectRespawn|SetJustRespawned true))))))

(event EventBeginPlay
  ;[1 1 0.4 1 36] Initialization
  (Variables|ObjectRespawn|SetJustRespawned true)
  (CallFunction|SetStreamingSystemRef)
  (Actor|Tick|SetActorTickEnabled false)
  (Variables|Default|SetShouldSimulatePhysics true))

(event EventPickup
  (params (ServerOwningCharacter :type Pawn%20Object%20Reference) (LocalOwningCharacter :type Pawn%20Object%20Reference) (LeftHand :type Boolean) (UserMesh :type Skeletal%20Mesh%20Component%20Object%20Reference) (SocketName :type Name :default "None") (MotionController :type Motion%20Controller%20Component%20Object%20Reference) (InstigatorReference :type Controller%20Object%20Reference))
  ;[1 0.4 0.4 1 36] Pickup Actor - only called by Server
  (Networking|SwitchHasAuthority
    (:Authority
      (Variables|Pickup|SetLeftHand LeftHand)
      (Variables|Default|SetShouldSimulatePhysics false)
      (Transformation|AttachComponentToComponent (Variables|Debug|GetStaticMeshComponent) UserMesh SocketName "KeepRelative" "KeepRelative" "KeepWorld" true)
      (Variables|Pickup|SetIsPickedUp true)
      (Variables|ObjectRespawn|SetJustRespawned false)
      (CallFunction|MulticastCancelRespawn)
      (bind _asvr_pawn (Utilities|Casting|CastToVR_Pawn ServerOwningCharacter)
        (:then
          (Variables|Default|SetUserReference _asvr_pawn))
        (:CastFailed
          _))
      (CallFunction|AdjusttoHand)
      (Audio|PlaySound2D (Variables|Default|GetSoundPickUp) 1.0 1.0 0.0 0 0)
      (Default|CallOnPickedUp self))))

(event EventDrop
  (params (LeftHand :type Boolean))
  ;[1 0.4 0.4 1 36] Drop Actor - only called by Server
  (Networking|SwitchHasAuthority
    (:Authority
      (Transformation|DetachFromComponent (Variables|Debug|GetStaticMeshComponent) "KeepRelative" "KeepRelative" "KeepWorld" true)
      (Variables|Default|SetShouldSimulatePhysics true)
      (Variables|Pickup|SetIsPickedUp false)
      (Variables|Default|SetUserReference 0))))

(fn ConstructionScript
  (bind _staticmeshcomponent (Variables|Debug|GetStaticMeshComponent))
  (for _array_element (Components|GetChildrenComponents _staticmeshcomponent false)
    (Transformation|AttachComponentToComponent _array_element _staticmeshcomponent "None" "KeepRelative" "KeepRelative" "KeepRelative" true)))

(fn BlinkObjectThenRespawn
  (bind _streamingsystemref (Variables|ObjectRespawn|GetStreamingSystemRef))
  (bind _blinkcounter (Variables|ObjectRespawn|GetBlinkCounter))
  (bind _initialtransform (Variables|ObjectRespawn|GetInitialTransform))
  (bind _returnvalue (Transformation|GetActorTransform _streamingsystemref))
  (Rendering|SetActorHiddenInGame (== (Math|Integer|%(Integer) (Variables|ObjectRespawn|GetBlinkCounter) 2) 0))
  (Math|Integer|IncrementInt _blinkcounter
    (:%20%20
      (if (> _blinkcounter 7)
        (Transformation|SetRelativeTransform (Variables|Debug|GetStaticMeshComponent) (Math|Transform|MakeTransform (Math|Transform|TransformLocation _returnvalue (.location _initialtransform)) (Math|Transform|TransformRotation _returnvalue (.rotation _initialtransform)) (.scale _initialtransform)) false true)
        (Utilities|Time|ClearandInvalidateTimerbyHandle (Variables|ObjectRespawn|GetBlinkHandle))
        (Networking|SwitchHasAuthority
          (:Authority
            (CallFunction|ResetStateforRespawn))
          (:Remote
            (Audio|PlaySoundatLocation (Variables|ObjectRespawn|GetRespawnedSound) (Transformation|GetActorLocation) "0, 0, 0" 1.0 1.0 0.0 0 0 0 0)))))))

(fn SetStreamingSystemRef
  (bind _returnvalue (Actor|GetActorOfClass "/Game/VR_Base/Streaming/BP_StreamingSystem.BP_StreamingSystem_C"))
  (Utilities|IsValid _returnvalue
    (:Is%20Valid
      (bind _output_get (Variables|ObjectRespawn|SetStreamingSystemRef _returnvalue))
      (EventDispatchers|BindEventtoOnNewLevelLoaded _output_get (EventDispatchers|CreateEvent :!event Custom|AttachToStreamingSystem))
      (if (not (Variables|/Game/VR_Base/Streaming/BP_StreamingSystem.BP_StreamingSystem_C|GetTransitionState _output_get))
        (CallFunction|AttachtoStreamingSystem "None")))
    (:Is%20Not%20Valid
      (Utilities|Time|SetTimerbyFunctionName 0 "SetStreamingSystemRef" 0.2))))

(fn OnRepIsPickedUp
  (CallFunction|OveridableonRepPickedUp))

(fn OveridableonRepPickedUp)

(fn OnRepShouldSimulatePhysics
  (Physics|SetSimulatePhysics (Variables|Debug|GetStaticMeshComponent) (Variables|Default|GetShouldSimulatePhysics)))

(fn AdjusttoHand
  (bind _lefthandrelativetransform (Variables|Pickup|GetLeftHandRelativeTransform))
  (bind _righthandrelativetransform (Variables|Pickup|GetRightHandRelativeTransform))
  ;[0 0 0] Adjust Cube to Hand-Offest
  (if (Variables|Pickup|GetLeftHand)
    (Transformation|SetRelativeLocationAndRotation (Variables|Debug|GetStaticMeshComponent) (.location _lefthandrelativetransform) (.rotation _lefthandrelativetransform) false false) ; Left Hand Gripping Offset
    (else
      (Transformation|SetRelativeLocationAndRotation (Variables|Debug|GetStaticMeshComponent) (.location _righthandrelativetransform) (.rotation _righthandrelativetransform) false false) ; Right Hand Gripping Offset
    )))

(fn CanbePickedUp
  (return true true true))

(fn GetGripType
  (return "NewEnumerator0"))

(fn GetHoldingHand
  (return (Variables|Pickup|GetLeftHand)))

(fn GetLocation
  (return "0, 0, 0"))

(fn GetPickupState
  (return (Variables|Pickup|GetIsPickedUp) false))

(fn GetUserReference
  (return (Variables|Default|GetUserReference)))