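; BP_Teleport is a VR interactable that makes every VR_Pawn execute a jump when activated with a teleport argument.
; Activate passes its string through ReportActivation for optional debug printing, then checks it for "Teleport" and prints an error otherwise.
; The jump uses a hard-coded vector, as the coordinate-parsing nodes are unconnected.
; BeginPlay caches the BP_StreamingSystem, though nothing here uses it.
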(event EventBeginPlay
  (bind _outactors (Actor|GetAllActorsOfClass "/Game/VR_Base/Streaming/BP_StreamingSystem.BP_StreamingSystem_C"))
  (Variables|Default|SetStreamingSystem (Utilities|Array|Get(acopy) _outactors)))

(event Collision|EventActorBeginOverlap
  (params (OtherActor :type Actor%20Object%20Reference)))

(event EventTick
  (params (DeltaSeconds :type Float%20%28single-precision%29))
  (|CallParentFunction DeltaSeconds) ; This node is disabled and will not be called.\nDrag off pins to build functionality.
)

(event EventActivate
  (params (Argument :type String) (User :type VR%20Pawn%20Object%20Reference))
  (bind _out (|ReportActivation Argument))
  (if (Utilities|String|Contains _out "Teleport")
    (bind _outactors (Actor|GetAllActorsOfClass "/Game/VR_Base/Character/VR_Pawn.VR_Pawn_C"))
    (for _array_element _outactors
      (Default|SRExecuteJump _array_element "200.000000,200.000000,0.000000"))
    (else
      (Utilities|PrintDebugMessage "Teleport_not_recognized!" "NewEnumerator2" true))))

(fn ConstructionScript
  (|CallParentFunction))