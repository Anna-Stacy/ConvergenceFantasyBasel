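; BP_MaleFemaleSelector is a VR interactable that switches the activating user's figure between male and female, and can also start a network connection.
; Activate logs its argument through a debug helper, then switches on it, reporting unrecognized selections.
; Gender choices call SRChangeUserFigureThroughPawn on the user.
; HOST (marked obsolete) and JOIN set the game instance's ShouldBeHost flag, then share the LaunchNetworkConnection call.
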(event EventBeginPlay)

(event Collision|EventActorBeginOverlap
  (params (OtherActor :type Actor%20Object%20Reference)))

(event EventTick
  (params (DeltaSeconds :type Float%20%28single-precision%29))
  (|CallParentFunction DeltaSeconds) ; This node is disabled and will not be called.\nDrag off pins to build functionality.
)

(event EventActivate
  (params (Argument :type String) (User :type VR%20Pawn%20Object%20Reference))
  (bind _returnvalue (Game|GetGameInstance))
  (bind _asvr_game_instance (Utilities|Casting|CastToVR_GameInstance _returnvalue))
  (bind _out (|ReportActivation Argument))
  (switch string _out
    (:Default
      (Utilities|PrintDebugMessage "Selection_not_recognized!" "NewEnumerator2" true))
    (:HOST
      ;[0.15 0.15 0.15 0.5] Obsolete - retained for future use as discretionary host
      (Variables|/Game/VR_Base/GameModes/VR_GameInstance.VR_GameInstance_C|SetShouldBeHost _asvr_game_instance true)
      (Default|LaunchNetworkConnection _asvr_game_instance (.AsVR%20Player%20Controller (Utilities|Casting|CastToVR_PlayerController (Game|GetPlayerController 0))) :!label _label))
    (:JOIN
      (Variables|/Game/VR_Base/GameModes/VR_GameInstance.VR_GameInstance_C|SetShouldBeHost _asvr_game_instance false)
      (goto _label))
    (:CHANGE_GENDER_MALE
      (Default|SRChangeUserFigureThroughPawn User true false false))
    (:CHANGE_GENDER_FEMALE
      (Default|SRChangeUserFigureThroughPawn User false false false))))

(fn ConstructionScript
  (|CallParentFunction))