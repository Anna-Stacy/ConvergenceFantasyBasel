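; Base actor for VR touch buttons that activates and deactivates instances of InteractionClass through BI_ActivateDeactivate.
; A VR_Pawn overlap starts per-tick fingertip checks against the sensor box, stopping when all fingers move away.
; Touch changes are routed through the pawn's SR calls, with a reactivation timeout and optional finger-driven movement clamped along the arrow direction.
; Replicated Activated state swaps the material, and child classes can override empty activation/deactivation hooks.
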(event OnComponentBeginOverlap(TouchCollisionBox)
  (params (OverlappedComponent :type Primitive%20Component%20Object%20Reference) (OtherActor :type Actor%20Object%20Reference) (OtherComp :type Primitive%20Component%20Object%20Reference) (OtherBodyIndex :type Integer) (bFromSweep :type Boolean) (SweepResult :type Hit%20Result%20Structure%20%28by%20ref%29))
  ;[0.4 1 0.4] Activate touch-checking on overlap with a child of VR_Character
  (if (not (Variables|Interaction|GetOverlapOngoing))
    (bind _asvr_pawn (Utilities|Casting|CastToVR_Pawn OtherActor)
      (:then
        (Variables|Interaction|SetOverlappingUser _asvr_pawn)
        (Variables|Interaction|SetOverlapOngoing true)
        (|ReportBeginOverlaponowner OtherActor OtherComp :!label _label))
      (:CastFailed
        (goto _label Non-VR_Character)))))

(event Custom|SR_Deactivate
  (bind _deactivationargument (Variables|Action|GetDeactivationArgument))
  ;[0.15 0.00851 0.1104 0.5] Comment
  ;;[1 0.4 0.4] Deactivate Button on Server
  (Variables|Interaction|SetActivated false)
  (Transformation|SetRelativeLocation (Variables|Default|GetTouchSensor) "0, 0, 0" false false) ; Reset TouchSensor position when no longer touched
  (CallFunction|CustomDeactivationFunction) ; Empty but Overridable
  (|ReportSR_Deactivate_4)
  ;;;[1 1 1] Execute deactivator function
  (for _array_element (Variables|Interaction|GetList%20of%20Interactors)
    (Class|BIActivateDeactivate|Deactivate(Message) _array_element _deactivationargument)
    (|ReportcallingDeactivate_4 _deactivationargument _array_element)))

(event Custom|SR_Activate
  (bind _activationargument (Variables|Action|GetActivationArgument))
  ;[0.15 0.00851 0.1104 0.5] Comment
  ;;[1 0.4 0.4] Activate Button on Server
  (Variables|Interaction|SetActivated true)
  (CallFunction|CustomActivationFunction) ; Empty but Overridable
  (|ReportSR_Activate_4)
  ;;;[1 1 1] Execute activator function
  (for _array_element (Variables|Interaction|GetList%20of%20Interactors)
    (Class|BIActivateDeactivate|Activate(Message) _array_element _activationargument)
    (|ReportcallingActivate_4 _activationargument _array_element)))

(event Custom|SR_MoveSensor
  (params (Location :type Vector))
  ;[0.15 0.00851 0.1104 0.5] Comment
  ;;[1 0.4 0.4] Move Sensor on Server
  (Transformation|SetWorldLocation (Variables|Default|GetTouchSensor) Location false false))

(event Custom|SR_Start%20Overlap
  (params (Pawn :type VR%20Pawn%20Object%20Reference))
  ;[0.15 0.00851 0.1104 0.5] Comment
  ;;[1 0.4 0.4] Activate Button on Server
  (|Reportstartoverlaponserver)
  (bind _output_get (Variables|Interaction|SetOverlappingUser Pawn))
  (Actor|SetOwner _output_get)
  (Variables|Interaction|SetOverlapOngoing true))

(event Custom|SR_Stop%20Overlap
  ;[0.15 0.00851 0.1104 0.5] Comment
  ;;[1 0.4 0.4] Stop Overlap on Server
  (Variables|Interaction|SetOverlapOngoing false)
  (|Reportstopoverlaponserver))

(event EventBeginPlay
  (bind (_box_center _box_extent) (|CalculateTouchboxextent))
  (bind _touchsensor (Variables|Default|GetTouchSensor))
  (bind _returnvalue (Transformation|GetWorldTransform _touchsensor))
  ;[1 1 0.4] Get Sensor World Location, Rotation and Extent (after child class has modified sensor size in construction script)
  (Variables|Movement|SetSensorWorldTransform (|SetScaletouniformly1-1-1 _returnvalue))
  (Transformation|SetWorldScale3D (Variables|Default|GetTouchCollisionBox) (+ (.Scale (Math|Transform|BreakTransform _returnvalue)) "0.800000,0.800000,0.800000"))
  (Variables|LookandFeel|SetTouchBoxCenter _box_center)
  (Variables|LookandFeel|SetBox%20Extent _box_extent)
  ;;[0.15 0.15 0.15 0.5] Find all activators / deactivators ... typically only one - but there could be more
  (bind _outactors (Actor|GetAllActorsOfClass (Variables|Action|GetInteractionClass)))
  (if (Utilities|Array|IsNotEmpty _outactors)
    (for _array_element _outactors
      (if (Utilities|DoesObjectImplementInterface _array_element "/Game/VR_Base/Activatables/BI_ActivateDeactivate.BI_ActivateDeactivate_C")
        (Utilities|Array|AddUnique (Variables|Interaction|GetList%20of%20Interactors) _array_element)
        (else
          (|Errornointerface))))
    (else
      (|Errornointeractionclass))))

(event EventTick
  (params (DeltaSeconds :type Float%20%28single-precision%29))
  (bind _touchingfingertip (Variables|Movement|GetTouchingFingerTip))
  (bind _pushabledirection (Variables|Movement|GetPushableDirection))
  ;[0.4 1 0.4] Only search, if there was an overlap with a child of VR_Character to save realtime.
  (if (Variables|Interaction|GetOverlapOngoing)
    ;;[1 1 1 0.5] Deactivate if user disappeared
    (Utilities|IsValid (Variables|Interaction|GetOverlappingUser)
      (:Is%20Valid
        (Utilities|FlowControl|Sequence
          (:then_0
            ;[0.4 1 0.4] Search Finger Tips of both Hands
            (Variables|Interaction|SetFinger%20is%20touching false)
            (Variables|Interaction|SetMinimalFingerDistance 2e+02) ; Used to end overlap if all fingers are far
            (CallFunction|CheckTouchingFingers true)
            (CallFunction|CheckTouchingFingers false))
          (:then_1
            ;[0.4 1 0.4] Activate if not yet activated
            (if (Math|Boolean|ANDBoolean (Variables|Interaction|GetFinger%20is%20touching) (not (Variables|Interaction|GetActivated)) (Variables|Default|GetButtonEnabled) (== (Variables|Action|GetTimeoutTickCounter) 0))
              (Variables|Action|SetTimeoutTickCounter (Variables|Action|GetTimeoutTicksBeforeReactivation))
              (Variables|Movement|SetFingerTipStartPosition _touchingfingertip)
              (|ReportSR_Activatethroughuser _touchingfingertip)
              (Niagara|SpawnSystematLocation "/Game/Roman_MovingObjects/Particles/ButtonBurst.ButtonBurst" (Transformation|GetWorldLocation (Variables|Default|GetTouchCollisionBox)) "0, 0, 0" "0.100000,0.100000,0.100000")
              ;;[1 1 1] Execute activator function
              (for _array_element (Variables|Interaction|GetList%20of%20Interactors)
                (Default|SRActivateThroughUser (Variables|Interaction|GetOverlappingUser) _array_element (Variables|Action|GetActivationArgument)))))
          (:then_2
            ;[0.4 1 0.4] Deactivate if it was activated
            (if (and (not (Variables|Interaction|GetFinger%20is%20touching)) (Variables|Interaction|GetActivated))
              (|ReportSR_Deactivatethroughuser)
              ;;[1 1 1] Execute activator function
              (for _array_element_2 (Variables|Interaction|GetList%20of%20Interactors)
                (Default|SRDeactivateThroughUser (Variables|Interaction|GetOverlappingUser) _array_element_2 (Variables|Action|GetActivationArgument)))))
          (:then_3
            ;[0.4 1 0.4] Move Button with Finger
            (if (and (Variables|Interaction|GetActivated) (Variables|LookandFeel|GetMoveWithFinger))
              (|ReportDot-Product_4 (Utilities|VectorXFloat _pushabledirection (Utilities|LimittoMax (Math|Vector|DotProduct (- (Variables|Movement|GetTouchingFingerTip) (Variables|Movement|GetFingerTipStartPosition)) (Variables|Movement|GetPushableDirection)) (Variables|LookandFeel|GetMaxButtonMovement%20in%20cm))) (Utilities|LimittoMax (Math|Vector|DotProduct (- (Variables|Movement|GetTouchingFingerTip) (Variables|Movement|GetFingerTipStartPosition)) (Variables|Movement|GetPushableDirection)) (Variables|LookandFeel|GetMaxButtonMovement%20in%20cm)) _pushabledirection)
              (Transformation|SetWorldLocation (Variables|Default|GetTouchSensor) (+ (Utilities|VectorXFloat _pushabledirection (Utilities|LimittoMax (Math|Vector|DotProduct (- (Variables|Movement|GetTouchingFingerTip) (Variables|Movement|GetFingerTipStartPosition)) (Variables|Movement|GetPushableDirection)) (Variables|LookandFeel|GetMaxButtonMovement%20in%20cm))) (.location (Variables|Movement|GetSensorWorldTransform))) false false)
              (|Reportbuttonmove (+ (Utilities|VectorXFloat _pushabledirection (Utilities|LimittoMax (Math|Vector|DotProduct (- (Variables|Movement|GetTouchingFingerTip) (Variables|Movement|GetFingerTipStartPosition)) (Variables|Movement|GetPushableDirection)) (Variables|LookandFeel|GetMaxButtonMovement%20in%20cm))) (.location (Variables|Movement|GetSensorWorldTransform))) (Utilities|LimittoMax (Math|Vector|DotProduct (- (Variables|Movement|GetTouchingFingerTip) (Variables|Movement|GetFingerTipStartPosition)) (Variables|Movement|GetPushableDirection)) (Variables|LookandFeel|GetMaxButtonMovement%20in%20cm)))))
          (:then_4
            ;[0.4 1 0.4] Decrement reactivation-timer and stop-overlap-and-checking if no finger is closer than 1m
            (if (== (Variables|Action|GetTimeoutTickCounter) 0)
              _
              (else
                (Math|Integer|DecrementInt (Variables|Action|GetTimeoutTickCounter)
                  (:%20%20
                    _))))
            (if (> (Variables|Interaction|GetMinimalFingerDistance) 1e+02)
              (Variables|Interaction|SetOverlapOngoing false)
              (|ReportDeactivation)))))
      (:Is%20Not%20Valid
        (CallFunction|SRStopOverlap)
        (Variables|Interaction|SetOverlapOngoing false)
        (Utilities|PrintDebugMessage "Overlapping ended" "NewEnumerator0" (Variables|Default|GetDebug))))))

(fn ConstructionScript
  (bind _touchsensor (Variables|Default|GetTouchSensor))
  (bind _returnvalue (Transformation|GetWorldTransform _touchsensor))
  (bind _scale (Math|Transform|BreakTransform _returnvalue))
  (bind _returnvalue_2 (Utilities|ChangeMtoCm _scale))
  ;[1 1 1] Set Initial  Material as deactivated
  (Rendering|Material|SetMaterial (Variables|Default|GetTouchSensor) 0 (Variables|LookandFeel|GetDeactivatedButtonMaterial))
  ;[1 1 1] Get Sensor World Location, Rotation and Extent (Scale is ignored)
  (Variables|Movement|SetSensorWorldTransform (|SetScaleto1 _returnvalue))
  (Transformation|SetWorldScale3D (Variables|Default|GetTouchCollisionBox) (+ _scale "1.000000,1.000000,1.000000"))
  (Variables|Default|SetMax%20Push%20Depth (* (.x _returnvalue_2) 4.0))
  (Variables|Default|SetMax%20Side%20Tolerance (/ (.y _returnvalue_2) 2.0))
  (Variables|Default|SetMax%20up-down%20Tolerance (/ (.z _returnvalue_2) 2.0))
  ;[1 1 1] Pushable Direction is set by the Arrow
  (Variables|Movement|SetPushableDirection (Math|Vector|GetForwardVector (Variables|Default|GetButtonMovementDirection)))
  ;[1 1 1] Debug Report
  (Rendering|SetVisibility (Variables|Default|GetTouchCollisionBox) (Variables|Default|GetDebug) false))

(fn OnRepActivated
  (bind _activated (Variables|Interaction|GetActivated))
  ;[1 1 1] Change Material when Activated/Deactivated
  (Rendering|Material|SetMaterial (Variables|Default|GetTouchSensor) 0 (select _activated (Variables|LookandFeel|GetActivatedButtonMaterial) (Variables|LookandFeel|GetDeactivatedButtonMaterial)))
  (Utilities|PrintDebugMessage (select _activated "OnRep Activated" "OnRep Deactivated") "NewEnumerator0" (Variables|Default|GetDebug)))

(fn CheckTouchingFingers
  (params (LeftHand :type Boolean))
  (Utilities|IsValid (Variables|Interaction|GetOverlappingUser)
    (:Is%20Valid
      (Utilities|PrintDebugMessage "Overlapping User is valid" "NewEnumerator0" (Variables|Default|GetDebug))
      ;[1 1 1] Check each finger, wheter it is touching (inside the box)
      (bind _fingertips (Class|BITouchInterface|GetFingerPositions(Message) (Variables|Interaction|GetOverlappingUser) LeftHand))
      (for (_array_element _array_index) _fingertips
        (if (|Checkfingerisininteractionbox _array_element)
          (Variables|Interaction|SetFinger%20is%20touching true)
          (Variables|Movement|SetTouchingFingerTip _array_element)
          (|ReporttouchingFinger _array_index LeftHand)
          (else
            ;[1 1 1] Update closest finger distance, if this finger is closer than the last recorded one
            (if (< (Math|Vector|Distance(Vector) _array_element (.location (Variables|Movement|GetSensorWorldTransform))) (Variables|Interaction|GetMinimalFingerDistance))
              (Variables|Interaction|SetMinimalFingerDistance (Math|Vector|Distance(Vector) _array_element (.location (Variables|Movement|GetSensorWorldTransform)))))))))
    (:Is%20Not%20Valid
      (Utilities|PrintDebugMessage "Overlapping User is not valid" "NewEnumerator0" (Variables|Default|GetDebug))))
  (return))

(fn CustomActivationFunction
  (return))

(fn CustomDeactivationFunction
  (return))