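; BP_ChangeLevel is a VR interactable that switches levels when activated with a selection argument.
; On BeginPlay it caches the first BP_StreamingSystem actor found in the world.
; Activate passes the argument through a debug-logging helper, maps "Level 1" or "Level 2" to a test map name, and calls SRChangeLevel on the streaming system.
; Unrecognized selections only print a debug error.
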(event EventBeginPlay
  (bind _outactors (Actor|GetAllActorsOfClass "/Game/VR_Base/Streaming/BP_StreamingSystem.BP_StreamingSystem_C"))
  (Variables|Default|SetStreamingSystem (Utilities|Array|Get(acopy) _outactors)))

(event Collision|EventActorBeginOverlap
  (params (OtherActor :type Actor%20Object%20Reference)))

(event EventTick
  (params (DeltaSeconds :type Float%20%28single-precision%29))
  (|CallParentFunction DeltaSeconds) ; This node is disabled and will not be called.\nDrag off pins to build functionality.
)

(event EventActivate
  (params (Argument :type String) (User :type VR%20Pawn%20Object%20Reference))
  (bind _out (|ReportActivation Argument))
  (switch string _out
    (:Default
      (Utilities|PrintDebugMessage "Selection_not_recognized!" "NewEnumerator2" true))
    (:Level_1
      (Variables|Default|SetNext%20Level%20Name "VR_TestLevel")
      (Development|PrintString (Utilities|String|Append "Change Level to " _out) :!label _label)
      (Default|SRChangeLevel (Variables|Default|GetStreamingSystem) (Variables|Default|GetNext%20Level%20Name) false false false true))
    (:Level_2
      (Variables|Default|SetNext%20Level%20Name "VR_TestLevel_2")
      (goto _label))))

(fn ConstructionScript
  (|CallParentFunction))